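; BP_Goal is a goal actor for a Pong-style game that awards a point to the opposing goal when the ball enters it.
; On BeginPlay it searches the other BP_Goal actors; if one still has player number 0, it takes number 1 and stores that goal as OtherPlatform.
; When BP_PingPongBall overlaps its Box, it increments the Score held on OtherPlatform.
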(event `self.ReceiveBeginPlay`
  (`|ExecutionSequence`
    (:`then_0`
      ;[1 1 1] назначение номера игрока
      (bind _outactors (`GameplayStatics.GetAllActorsOfClass` "BP_Goal_C"))
      (for _array_element _outactors
        (if (== _array_element self)
          _
          (elif (== (`/Game/PinPong/Blueprints/PinPong/BP_Goal.NumberPlayer` _array_element) 0)
            (set `self.NumberPlayer` 1)
            (set `self.OtherPlatform` _array_element)))))))

(event `self.Box.OnComponentBeginOverlap`
  (params (OverlappedComponent :type "PrimitiveComponent Object Reference") (OtherActor :type "Actor Object Reference") (OtherComp :type "PrimitiveComponent Object Reference") (OtherBodyIndex :type Integer) (bFromSweep :type Boolean) (SweepResult :type "HitResult Structure (by ref)"))
  (bind _otherplatform (`self.OtherPlatform`))
  ;[1 1 1] пополнение очков у ворот
  (if (== OtherActor "/Game/PinPong/Blueprints/PinPong/BP_PingPongBall.BP_PingPongBall")
    (set `/Game/PinPong/Blueprints/PinPong/BP_Goal.Score` (+ (`/Game/PinPong/Blueprints/PinPong/BP_Goal.Score` _otherplatform) 1) _otherplatform)))

(fn `UserConstructionScript`)